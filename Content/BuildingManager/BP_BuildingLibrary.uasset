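; Building helper library that creates an animated exploded view of a named building's floors and looks up its floor group.
; BuildlingBoom gets the child actors grouped under the building name, cancels their running tweens, then tweens each upward from its current location with a larger lift per index.
; In reverse, it tweens each actor back to the InitLocation stored on its FloorComponent.
; GetBuildingFloor returns the actor group for that name.
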(fn BuildlingBoom
  (params (BuildingName :type String) (bReverse :type Boolean))
  (bind _values (Utilities|Map|Values (Class|ActorLibrary|GetGroupActorChildMap 0 BuildingName)))
  (for (_array_element _array_index) _values
    (Class|TweenManagerActor|DeleteAllTweensbyObject _array_element "Any")
    (Class|TweenVectorStandardFactory|CreateTweenMoveActorto 0 _array_element (select bReverse (Variables|/Script/ExtensionClass.FloorComponent|GetInitLocation (Actor|GetComponentbyClass _array_element "/Script/ExtensionClass.FloorComponent")) (Math|Vector|MakeVector (.x (Transformation|GetActorLocation _array_element)) (.y (Transformation|GetActorLocation _array_element)) (+ (.z (Transformation|GetActorLocation _array_element)) (+ (* _array_index 5e+02) 3e+03)))) 1.0 "Linear")))

(fn GetBuildingFloor
  (params (BuildingName :type String))
  (return (Class|ActorLibrary|GetActorGroup 0 BuildingName)))